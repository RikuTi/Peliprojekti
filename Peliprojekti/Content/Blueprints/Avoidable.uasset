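; Avoidable is a hazard actor that drains the player character's LifeForce on contact.
; When its RenderComponent overlaps BB_MyCharacter, matched by display name and then cast, it subtracts Effect from LifeForce, clamping at zero.
; A non-lethal hit also hides the render component and overrides Speed with a fixed value.
; BeginPlay caches the initial Speed in DefaultSpeed, though nothing here moves the actor or restores that value.
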(event OnComponentBeginOverlap(RenderComponent)
  (params (OverlappedComponent :type Primitive%20Component%20Object%20Reference) (OtherActor :type Actor%20Object%20Reference) (OtherComp :type Primitive%20Component%20Object%20Reference) (OtherBodyIndex :type Integer) (bFromSweep :type Boolean) (SweepResult :type Hit%20Result%20Structure%20%28by%20ref%29))
  (if (Utilities|Enum|Equal(Enum) (Utilities|GetDisplayName OtherActor) "BB_MyCharacter")
    (bind _asbb_my_character (Utilities|Casting|CastToBB_MyCharacter OtherActor))
    (if (> (Variables|/Game/Blueprints/BB_MyCharacter.BB_MyCharacter_C|GetLifeForce _asbb_my_character) 0.0)
      (if (> (- (Variables|/Game/Blueprints/BB_MyCharacter.BB_MyCharacter_C|GetLifeForce _asbb_my_character) (Variables|Default|GetEffect)) 0.0)
        (Variables|/Game/Blueprints/BB_MyCharacter.BB_MyCharacter_C|SetLifeForce _asbb_my_character (- (Variables|/Game/Blueprints/BB_MyCharacter.BB_MyCharacter_C|GetLifeForce _asbb_my_character) (Variables|Default|GetEffect)))
        (Rendering|SetVisibility (Variables|Default|GetRenderComponent) false false)
        (Variables|Default|SetSpeed 3e+02)
        (else
          (Variables|/Game/Blueprints/BB_MyCharacter.BB_MyCharacter_C|SetLifeForce _asbb_my_character 0.0))))))

(event EventBeginPlay
  (Variables|Default|SetdefaultSpeed (Variables|Default|GetSpeed)))

(event Collision|EventActorBeginOverlap
  (params (OtherActor :type Actor%20Object%20Reference)))

(event EventTick
  (params (DeltaSeconds :type Float%20%28single-precision%29)))

(fn ConstructionScript)