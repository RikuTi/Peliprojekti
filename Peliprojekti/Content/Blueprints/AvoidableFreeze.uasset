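; AvoidableFreeze is a hazard that applies a negative effect to BB_MyCharacter on overlap.
; A display-name check and cast identify the player, skipping any already under a negative effect.
; Otherwise it flags the effect, timestamps it on the character, halves the player's scale, hides its render component and overrides its own Speed.
; BeginPlay caches the default Speed, but nothing here restores it or ends the effect.
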(event OnComponentBeginOverlap(RenderComponent)
  (params (OverlappedComponent :type Primitive%20Component%20Object%20Reference) (OtherActor :type Actor%20Object%20Reference) (OtherComp :type Primitive%20Component%20Object%20Reference) (OtherBodyIndex :type Integer) (bFromSweep :type Boolean) (SweepResult :type Hit%20Result%20Structure%20%28by%20ref%29))
  (if (Utilities|Enum|Equal(Enum) (Utilities|GetDisplayName OtherActor) "BB_MyCharacter")
    (bind _asbb_my_character (Utilities|Casting|CastToBB_MyCharacter OtherActor))
    (if (not (Variables|/Game/Blueprints/BB_MyCharacter.BB_MyCharacter_C|GetIsNegativeEffectActive _asbb_my_character))
      (Variables|/Game/Blueprints/BB_MyCharacter.BB_MyCharacter_C|SetIsNegativeEffectActive _asbb_my_character true)
      (Variables|/Game/Blueprints/BB_MyCharacter.BB_MyCharacter_C|SetNegativeEffectStartTime _asbb_my_character (Utilities|Time|GetGameTimeinSeconds))
      (Rendering|SetVisibility (Variables|Default|GetRenderComponent) false false)
      (Variables|Default|SetSpeed 3e+02)
      (Transformation|SetWorldScale3D (Variables|/Script/Engine.Actor|GetRootComponent _asbb_my_character) "0.500000,0.500000,0.500000"))))

(event EventBeginPlay
  (Variables|Default|SetdefaultSpeed (Variables|Default|GetSpeed)))

(event Collision|EventActorBeginOverlap
  (params (OtherActor :type Actor%20Object%20Reference)))

(event EventTick
  (params (DeltaSeconds :type Float%20%28single-precision%29)))

(fn ConstructionScript)