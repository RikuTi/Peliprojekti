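; CollectiblesPool is an actor that pools collectibles and scrolls them along negative X.
; CreateCollectible spawns one at the start X with random height and speed, up to a maximum count.
; UpdateCollectibles moves each by its speed, recycling those past the mirrored X bound as visible, with new height and speed.
; Random speed bounds depend on elapsed game time; neither function is called within this Blueprint.
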(event EventBeginPlay)

(event Collision|EventActorBeginOverlap
  (params (OtherActor :type Actor%20Object%20Reference)))

(event EventTick
  (params (DeltaSeconds :type Float%20%28single-precision%29)))

(fn ConstructionScript)

(fn CreateCollectible
  (if (< (Variables|Default|GetnumberOfCollectibles) (Variables|Default|GetmaxNumberofCollectibles))
    (bind _returnvalue (Game|SpawnActorfromClass "/Game/Blueprints/Colleticble.Colleticble_C" (Math|Transform|MakeTransform (Math|Vector|MakeVector (Variables|Default|GetcollectibleStartX) 0.0 (Math|Random|RandomFloatinRange -4e+02 1e+03))) "Undefined" 0 0))
    (Variables|/Game/Blueprints/Colleticble.Colleticble_C|SetSpeed _returnvalue (Math|Random|RandomFloatinRange (/ (Variables|/Game/Blueprints/Colleticble.Colleticble_C|GetSpeed _returnvalue) (/ (Utilities|Time|GetGameTimeinSeconds) 1e+01)) (Variables|/Game/Blueprints/Colleticble.Colleticble_C|GetSpeed _returnvalue)))
    (Utilities|Array|Insert (Variables|Default|GetthePool) _returnvalue (Variables|Default|GetnumberOfCollectibles))
    (Math|Integer|IncrementInt (Variables|Default|GetnumberOfCollectibles))))

(fn UpdateCollectibles
  (for (_array_element _array_index) (Variables|Default|GetthePool)
    (LocalVariables|SetarrayElement _array_element)
    (LocalVariables|SetarrayIndex _array_index)
    (if (< (.X (Math|Vector|BreakVector (Transformation|GetWorldLocation (Variables|/Script/Engine.Actor|GetRootComponent _array_element)))) (- 0.0 (Variables|Default|GetcollectibleStartX)))
      (Transformation|SetWorldLocation (Variables|/Script/Engine.Actor|GetRootComponent (LocalVariables|GetarrayElement)) (Math|Vector|MakeVector (Variables|Default|GetcollectibleStartX) 0.0 (Math|Random|RandomFloatinRange -4e+02 4e+02)) false false)
      (Rendering|SetVisibility (Variables|/Script/Engine.Actor|GetRootComponent (LocalVariables|GetarrayElement)) true false)
      (Variables|/Game/Blueprints/Colleticble.Colleticble_C|SetSpeed (LocalVariables|GetarrayElement) (Math|Random|RandomFloatinRange (/ (Variables|/Game/Blueprints/Colleticble.Colleticble_C|GetdefaultSpeed (LocalVariables|GetarrayElement)) (/ (Utilities|Time|GetGameTimeinSeconds) 1e+01)) (Variables|/Game/Blueprints/Colleticble.Colleticble_C|GetdefaultSpeed (LocalVariables|GetarrayElement))))
      (else
        (bind _ascolleticble (Utilities|Casting|CastToColleticble _array_element))
        (Transformation|AddActorWorldOffset _array_element (Math|Vector|MakeVector (- 0.0 (Variables|/Game/Blueprints/Colleticble.Colleticble_C|GetSpeed _ascolleticble)) 0.0 0.0))))))